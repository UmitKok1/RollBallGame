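; Base pickup actor that awards Points to a BallPawn on sphere overlap and counts toward its goal targets, except for Explosive subclasses.
; Pickup plays a sound and particles, then either swaps the mesh for a PickupText score widget, seeded on BeginPlay, or destroys itself immediately.
; The overlap event also destroys the actor after a short delay, whatever actor overlapped it.
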(event OnComponentBeginOverlap(Sphere)
  (params (OverlappedComponent :type Primitive%20Component%20Object%20Reference) (OtherActor :type Actor%20Object%20Reference) (OtherComp :type Primitive%20Component%20Object%20Reference) (OtherBodyIndex :type Integer) (bFromSweep :type Boolean) (SweepResult :type Hit%20Result%20Structure%20%28by%20ref%29))
  (CallFunction|OnPickUp OtherActor)
  (Utilities|FlowControl|Delay 0.75)
  (Actor|DestroyActor))

(event EventBeginPlay
  (bind _aspickup_text (Utilities|Casting|CastToPickupText (UserInterface|GetUserWidgetObject (Variables|Default|GetWidget))))
  (Variables|/Game/Blueprints/Pickup/PickupText.PickupText_C|SetScoreValue _aspickup_text (Variables|Default|GetPoints)))

(fn ConstructionScript)

(fn OnPickUp
  (params (Object :type Object%20Object%20Reference))
  (bind _asball_pawn (Utilities|Casting|CastToBallPawn Object))
  (Utilities|Casting|CastToExplosive self
    (:then
      _)
    (:CastFailed
      (Default|IncrementGoalTargets _asball_pawn)))
  (Default|IncrementScore _asball_pawn (Variables|Default|GetPoints))
  (Audio|PlaySound2D (Variables|Default|GetOnPickupSound) 1.0 1.0 0.0 0 0)
  (Effects|SpawnEmitteratLocation (Variables|Default|GetOnPickupParticles) (Transformation|GetActorLocation))
  (if (Variables|Default|GetUseNumberWidget)
    (Rendering|SetVisibility (Variables|Default|GetWidget) true false)
    (Rendering|SetVisibility (Variables|Default|GetStaticMesh) false false)
    (else
      (Actor|DestroyActor))))