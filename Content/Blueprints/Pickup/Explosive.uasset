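; Explosive hazard pickup that blasts the player's BallPawn with a radial impulse from just below itself when picked up.
; Configures the parent pickup with explosion effects, zero points and no number widget, and plays a spark sound from BeginPlay.
; Binds DestroySelf to the player's destroy-hazards event, which shows a sparkle, waits briefly, silences the sparks and removes the actor.
; Pickup silences the sparks, then defers to the parent logic.
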(event Custom|DestroySelf
  (Effects|SpawnEmitteratLocation "/Game/InfinityBladeEffects/Effects/FX_Treasure/Gold_Bag/P_GoldSparkle_Bag_Pickup.P_GoldSparkle_Bag_Pickup" (Transformation|GetActorLocation))
  (Utilities|FlowControl|Delay 0.75)
  (Components|Activation|SetActive (Variables|Default|GetSparksSound) false false)
  (Actor|DestroyActor))

(event EventBeginPlay
  (Variables|Default|SetUseNumberWidget false)
  (Variables|Default|SetOnPickupSound "/Game/StarterContent/Audio/Explosion01.Explosion01")
  (Variables|Default|SetOnPickupParticles "/Game/StarterContent/Particles/P_Explosion.P_Explosion")
  (Variables|Default|SetPoints 0)
  (bind _returnvalue (Audio|SpawnSoundatLocation "/Game/StarterContent/Audio/Fire_Sparks01_Cue.Fire_Sparks01_Cue" (Transformation|GetActorLocation) "0, 0, 0" 1.0 1.0 0.0 0 0))
  (Variables|Default|SetSparksSound _returnvalue)
  (|CallParentFunction)
  (EventDispatchers|BindEventtoDestroyHazards (.AsBall%20Pawn (Utilities|Casting|CastToBallPawn (Game|Player|GetPlayerPawn 0))) (delegate Custom|DestroySelf)))

(event EventOnPickUp
  (params (Object :type Object%20Object%20Reference))
  (bind _returnvalue (Transformation|GetActorLocation))
  (bind (_x _y _z) (Math|Vector|BreakVector _returnvalue))
  (bind _asball_pawn (Utilities|Casting|CastToBallPawn Object))
  (Physics|AddRadialImpulse (Variables|/Game/Blueprints/Character/BallPawn.BallPawn_C|GetBallMesh _asball_pawn) (Math|Vector|MakeVector _x _y (+ _z -75.0)) 5e+03 2e+03 "RIF_Constant" true)
  (Development|PrintString "Hello")
  (Components|Activation|SetActive (Variables|Default|GetSparksSound) false false)
  (|CallParentFunction Object))

(fn ConstructionScript
  (|CallParentFunction))