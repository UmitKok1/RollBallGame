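; Pressure button actor that responds when a BallPawn enters or leaves its overlap sphere.
; On overlap begin it plays a pickup sound and runs a timeline that offsets the button's Z from its starting world location.
; On overlap end it reverses the timeline, with the same update restoring the button's height.
; It also loops over an AffectedActors list on press, but the loop body is empty.
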(event OnComponentBeginOverlap(OverlapSphere)
  (params (OverlappedComponent :type Primitive%20Component%20Object%20Reference) (OtherActor :type Actor%20Object%20Reference) (OtherComp :type Primitive%20Component%20Object%20Reference) (OtherBodyIndex :type Integer) (bFromSweep :type Boolean) (SweepResult :type Hit%20Result%20Structure%20%28by%20ref%29))
  (bind _initialbuttonlocation (Variables|Default|GetInitialButtonLocation))
  (bind (_x _y _z) (Math|Vector|BreakVector _initialbuttonlocation))
  (Utilities|Casting|CastToBallPawn OtherActor)
  (Audio|PlaySound2D "/Game/Retro_8Bit_Sounds/Collectables/Cues/retro_collect_pickup_item_08_Cue.retro_collect_pickup_item_08_Cue" 1.0 1.0 0.0 0 0)
  (for _array_element (Variables|Default|GetAffectedActors)
    _)
  (bind _buttonelevation (Timeline|ButtonTimeline Play)
    (:Update
      (Transformation|SetWorldLocation (Variables|Default|GetButton) (Math|Vector|MakeVector _x _y (+ _z _buttonelevation)) false false))))

(event OnComponentEndOverlap(OverlapSphere)
  (params (OverlappedComponent :type Primitive%20Component%20Object%20Reference) (OtherActor :type Actor%20Object%20Reference) (OtherComp :type Primitive%20Component%20Object%20Reference) (OtherBodyIndex :type Integer))
  (bind _initialbuttonlocation (Variables|Default|GetInitialButtonLocation))
  (bind (_x _y _z) (Math|Vector|BreakVector _initialbuttonlocation))
  (Utilities|Casting|CastToBallPawn OtherActor)
  (bind _buttonelevation (Timeline|ButtonTimeline Reverse)
    (:Update
      (Transformation|SetWorldLocation (Variables|Default|GetButton) (Math|Vector|MakeVector _x _y (+ _z _buttonelevation)) false false))))

(event EventBeginPlay
  (Variables|Default|SetInitialButtonLocation (Transformation|GetWorldLocation (Variables|Default|GetButton))))

(fn ConstructionScript)